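; Enemy mech AI that wanders, chases the player on sight and fires a rifle, with a camera-facing health bar.
; Patrol loops AIMoveTo to random nearby points, while PawnSensing triggers a chase that ends in Fire.
; Fire uses a cooldown-gated line trace to apply damage with montage and effects.
; Lethal damage triggers ragdoll, increments player score, plays explosions, drops a health pickup and destroys the mech.
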(event `self.ReceiveBeginPlay`
  ;[1 1 1] Begin
  (`|ExecutionSequence`
    (:`then_0`
      (bind _aswbp_health_bar (cast `/Game/ThirdPerson/UserInterface/WBP_HealthBar` (`WidgetComponent.GetWidget` (`self.Widget`))))
      (set `self.WBP Health Bar` _aswbp_health_bar))
    (:`then_1`
      (`KismetSystemLibrary.Delay` 0.02)
      (`self.Patrol`))))

(event `self.ReceiveTick`
  (params (DeltaSeconds :type "Float (single-precision)"))
  ;[1 1 1] Health_Display
  (`/Engine/EditorBlueprintResources/StandardMacros.IsValid` (`self.WBP Health Bar`)
    (:`Is Valid`
      (`SceneComponent.K2_SetWorldRotation` (`self.Widget`) (`KismetMathLibrary.FindLookAtRotation` (`self.K2_GetActorLocation`) (`self.K2_GetActorLocation` (`GameplayStatics.GetPlayerCameraManager` 0))) false false)
      (`/Game/ThirdPerson/UserInterface/WBP_HealthBar.SetHealthBar` (`self.WBP Health Bar`) (`self.Health`) (`self.MaxHealth`)))))

(event `ChasePlayer`
  (params (TargetActor :type "Actor Object Reference"))
  ;[1 1 1] Chase
  (`|AIMoveTo` self (0.0 0.0 0.0) TargetActor 300.0
    (:`OnSuccess`
      _)
    (:`OnFail`
      _))
  (if (not (`self.IsDead`))
    (`self.Fire`)))

(event `Patrol`
  ;[1 1 1] Patrol
  (`|AIMoveTo` self (`NavigationSystemV1.K2_GetRandomReachablePointInRadius` (`self.K2_GetActorLocation`) 300.0 null null) null
    (:`OnSuccess`
      _)
    (:`OnFail`
      _))
  (if (not (`self.IsDead`))
    (`self.Patrol`)))

(event `self.PawnSensing.OnSeePawn`
  (params (Pawn :type "Pawn Object Reference"))
  ;[1 1 1] Detect
  (bind _asbp_third_person_character (cast `/Game/ThirdPerson/Blueprints/BP_ThirdPersonCharacter` Pawn))
  (`self.ChasePlayer` _asbp_third_person_character))

(event `self.ReceiveAnyDamage`
  (params (Damage :type "Float (single-precision)") (DamageType :type "DamageType Object Reference") (InstigatedBy :type "Controller Object Reference") (DamageCauser :type "Actor Object Reference"))
  (bind _returnvalue (`self.K2_GetActorLocation`))
  (bind _mesh (`self.Mesh`))
  ;[1 1 1] Damage
  (if (not (`self.IsDead`))
    (set `self.Health` (- (`self.Health`) Damage))
    (set `self.IsDead` (<= (`self.Health`) 0.0))
    (if (`self.IsDead`)
      (`KismetSystemLibrary.Delay` 0.5)
      (`PrimitiveComponent.SetSimulatePhysics` (`self.Mesh`) true)
      (`SceneComponent.SetVisibility` (`self.Widget`) false false)
      (`SceneComponent.SetVisibility` (`self.EnemyName`) false false)
      (`GameplayStatics.SpawnEmitterAttached` "/Game/Realistic_Starter_VFX_Pack_Vol2/Particles/Destruction/P_Destruction_Electric.P_Destruction_Electric" _mesh)
      (`GameplayStatics.PlaySoundAtLocation` "/Game/SFX/shock.shock" _returnvalue (struct) 1.0 1.0 0.0 null null null null)
      (`|ExecutionSequence`
        (:`then_0`
          (bind _asbp_third_person_character (cast `/Game/ThirdPerson/Blueprints/BP_ThirdPersonCharacter` (`GameplayStatics.GetPlayerCharacter` 0)))
          (`/Engine/EditorBlueprintResources/StandardMacros.IncrementInt` (`/Game/ThirdPerson/Blueprints/BP_ThirdPersonCharacter.Score` _asbp_third_person_character)))
        (:`then_1`
          (`GameplayStatics.SpawnEmitterAttached` "/Game/StarterContent/Particles/P_Fire.P_Fire")
          (`KismetSystemLibrary.Delay` 0.5)
          (`GameplayStatics.SpawnEmitterAttached` "/Game/Realistic_Starter_VFX_Pack_Vol2/Particles/Explosion/P_Explosion_Big_B.P_Explosion_Big_B" _mesh)
          (`GameplayStatics.PlaySoundAtLocation` "/Game/StarterContent/Audio/Explosion01.Explosion01" _returnvalue (struct) 1.0 1.0 0.0 null null null null)
          (`self.DropItem`)
          (`KismetSystemLibrary.Delay` 1.5)
          (`self.K2_DestroyActor`))))))

(event `Fire`
  (bind _returnvalue (`KismetMathLibrary.RandomFloatInRange` 0.1 0.5))
  (bind _rifle (`self.Rifle`))
  (bind _returnvalue_location (`KismetMathLibrary.BreakTransform` (`SceneComponent.GetSocketTransform` _rifle "None" "RTS_World")))
  (bind _returnvalue_location_2 (`KismetMathLibrary.BreakTransform` (`SceneComponent.GetSocketTransform` _rifle "Muzzle" "RTS_Component")))
  ;[1 1 1] Shoot
  (if (and (not (`self.IsDead`)) (not (`/Game/ThirdPerson/Blueprints/BP_ThirdPersonCharacter.IsDead` (stale `self.PawnSensing.OnSeePawn` _asbp_third_person_character))))
    (`/Engine/EditorBlueprintResources/StandardMacros.DoOnce` false :!label _label
      (:`Completed`
        (`|ExecutionSequence`
          (:`then_0`
            (`|PlayMontage` (`self.Mesh`) "/Game/Characters/AnimationShooter/Fire_Rifle_Ironsights_Montage.Fire_Rifle_Ironsights_Montage"
              (:`then`
                (`GameplayStatics.PlaySoundAtLocation` "/Game/SFX/Weapon_Fire_Start.Weapon_Fire_Start" _returnvalue_location (struct) 1.0 1.0 0.0 null null null null)
                (`GameplayStatics.SpawnEmitterAttached` "/Game/InfinityBladeEffects/Effects/FX_Monsters/FX_Monster_Chicken/P_ChickenMaster_MuzzleFlash_01.P_ChickenMaster_MuzzleFlash_01" _rifle "None" _returnvalue_location_2 (struct :`Yaw` 90.0) (0.2 0.2 0.2))
                (bind (_outhit _returnvalue_2) (`KismetSystemLibrary.LineTraceSingle` _returnvalue_location (+ _returnvalue_location (* (`SceneComponent.GetRightVector` (`self.Mesh`)) 3000.0)) "TraceTypeQuery1"))
                (if _returnvalue_2
                  (bind (_bblockinghit _binitialoverlap _time _distance _location _impactpoint _normal _impactnormal _physmat _hitactor) (`GameplayStatics.BreakHitResult` _outhit))
                  (`GameplayStatics.SpawnEmitterAtLocation` "/Game/StarterContent/Particles/P_Explosion.P_Explosion" _impactpoint (struct) (`KismetMathLibrary.Conv_DoubleToVector` _returnvalue))
                  (`GameplayStatics.SpawnEmitterAtLocation` "/Game/Realistic_Starter_VFX_Pack_Vol2/Particles/Destruction/P_Destruction_Electric.P_Destruction_Electric" (+ _returnvalue _impactpoint) (struct) (`KismetMathLibrary.Conv_DoubleToVector` _returnvalue))
                  (`GameplayStatics.ApplyDamage` _hitactor 10.0)))))
          (:`then_1`
            (`KismetSystemLibrary.Delay` 0.2)
            (goto _label :!via `Reset`)))))))

(event `DropItem`
  (bind _returnvalue (`self.K2_GetActorLocation`))
  ;[1 1 1] Damage
  (bind _outhit (`KismetSystemLibrary.LineTraceSingle` _returnvalue (+ _returnvalue (0.0 0.0 -200.0)) "TraceTypeQuery1" false (`|MakeArray` (`GameplayStatics.GetPlayerCharacter` 0) :!type "Actor Object Reference")))
  (`|SpawnActorFromClass` "/Game/ThirdPerson/Blueprints/BP_Health.BP_Health_C" (`KismetMathLibrary.MakeTransform` (`.Location` (`GameplayStatics.BreakHitResult` _outhit))) "AdjustIfPossibleButDontSpawnIfColliding" "MultiplyWithRoot" null null))

(fn `UserConstructionScript`)