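; Enemy character that hunts the player in the survival game and restarts the level when it catches them.
; On BeginPlay it casts the player pawn to BP_MainChar, sets its own walk speed and fires the ChasePlayer event.
; ChasePlayer issues a single AIMoveTo toward that actor and reopens the current level on success.
; A failed move has no handling or retry, and Tick is unused.
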(event `self.ReceiveBeginPlay`
  (bind _asbp_main_char (cast `/Game/SurvivalGame/Blueprint/BP_MainChar` (`GameplayStatics.GetPlayerCharacter` 0)))
  (set `CharacterMovementComponent.MaxWalkSpeed` 200.0 (`self.CharacterMovement`))
  (`self.ChasePlayer` _asbp_main_char))

(event `ChasePlayer`
  (params (TargetActor :type "Actor Object Reference"))
  (`|AIMoveTo` self (0.0 0.0 0.0) TargetActor
    (:`OnSuccess`
      (bind _returnvalue (`GameplayStatics.GetCurrentLevelName` true))
      (`GameplayStatics.OpenLevel` (`KismetStringLibrary.Conv_StringToName` _returnvalue)))))

(fn `UserConstructionScript`)